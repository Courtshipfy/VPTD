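; Player character for a 2D top-down build-and-attack game, moved by axis input and animated with Paper2D flipbooks.
; Tick picks and mirrors the flipbook from FaceDirection and build state, and yaws the hidden Gun toward the cursor when IsGun is set.
; E swaps the Gun to a book while held, flags GameMode building, and alternately raises or lowers the selection widget.
; Mouse and F set attack and select flags; directional gun-sprite logic is disconnected.
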(event `Key|LeftMouseButton`
  (params (Key :type "Key Structure"))
  ;[1 1 1] AttackSystem
  (:`Pressed`
    (if (`self.AttackMode?`)
      (set `self.Attacking?` true)))
  (:`Released`
    (set `self.Attacking?` false)))

(event `InputAxis|Vertical Moving`
  (params (AxisValue :type "Float (single-precision)"))
  ;[1 1 1] Find FaceDirection
  (`self.AddMovementInput` (0.0 1.0 0.0) AxisValue)
  (`/Engine/EditorBlueprintResources/StandardMacros.CompareFloat` AxisValue
    (:`>`
      (`/Engine/EditorBlueprintResources/StandardMacros.CompareFloat` (stale `InputAxis|Horizontal Moving` AxisValue)
        (:`>`
          (set `self.FaceDirection` "NewEnumerator7"))
        (:`==`
          (set `self.FaceDirection` "NewEnumerator1"))
        (:`<`
          (set `self.FaceDirection` "NewEnumerator6"))))
    (:`==`
      (`/Engine/EditorBlueprintResources/StandardMacros.CompareFloat` (stale `InputAxis|Horizontal Moving` AxisValue)
        (:`>`
          (set `self.FaceDirection` "NewEnumerator3"))
        (:`==`
          (set `self.FaceDirection` "NewEnumerator8"))
        (:`<`
          (set `self.FaceDirection` "NewEnumerator2"))))
    (:`<`
      (`/Engine/EditorBlueprintResources/StandardMacros.CompareFloat` (stale `InputAxis|Horizontal Moving` AxisValue)
        (:`>`
          (set `self.FaceDirection` "NewEnumerator5"))
        (:`==`
          (set `self.FaceDirection` "NewEnumerator0"))
        (:`<`
          (set `self.FaceDirection` "NewEnumerator4"))))))

(event `InputAxis|Horizontal Moving`
  (params (AxisValue :type "Float (single-precision)"))
  ;[1 1 1] Find FaceDirection
  (`self.AddMovementInput` (1.0 0.0 0.0) AxisValue))

(event `Key|E`
  (params (Key :type "Key Structure"))
  (bind _gun (`self.Gun`))
  (:`Pressed`
    (`PaperSpriteComponent.SetSprite` _gun "/Game/Assets/Weapon/Book_Sprite.Book_Sprite")
    (`PaperSpriteComponent.SetSpriteColor` _gun (struct :`A` 0.621))
    (bind _asbp_vptd_game_mode (cast `/Game/BP_VPTD_GameMode` (`GameplayStatics.GetGameMode`)))
    (set `/Game/BP_VPTD_GameMode.isBuilding` true _asbp_vptd_game_mode)
    (`/Engine/EditorBlueprintResources/StandardMacros.FlipFlop`
      (:`A`
        (bind _foundwidgets (`WidgetBlueprintLibrary.GetAllWidgetsOfClass` "/Game/Blueprint/Widgets_BP/Attributes_Widget.Attributes_Widget_C"))
        (`/Game/Blueprint/Widgets_BP/Attributes_Widget.UpSelectWindow` (`|GetArrayItem` _foundwidgets))
        (set `self.isBuilding` true))
      (:`B`
        (bind _foundwidgets_2 (`WidgetBlueprintLibrary.GetAllWidgetsOfClass` "/Game/Blueprint/Widgets_BP/Attributes_Widget.Attributes_Widget_C"))
        (`/Game/Blueprint/Widgets_BP/Attributes_Widget.DownSelectWindow` (`|GetArrayItem` _foundwidgets_2))
        (set `self.isBuilding` false))))
  (:`Released`
    (`PaperSpriteComponent.SetSprite` _gun "/Game/Assets/Weapon/cannon_side_Sprite.cannon_side_Sprite")
    (`PaperSpriteComponent.SetSpriteColor` _gun (struct :`R` 1.0 :`G` 1.0 :`B` 1.0 :`A` 1.0))
    (bind _asbp_vptd_game_mode_2 (cast `/Game/BP_VPTD_GameMode` (`GameplayStatics.GetGameMode`)))
    (set `/Game/BP_VPTD_GameMode.isBuilding` false _asbp_vptd_game_mode_2)))

(event `Key|F`
  (params (Key :type "Key Structure"))
  (:`Pressed`
    (set `self.isSelected` true))
  (:`Released`
    (set `self.isSelected` false)))

(event `self.ReceiveTick`
  (params (DeltaSeconds :type "Float (single-precision)"))
  (bind (_returnvalue_roll _returnvalue_pitch) (`KismetMathLibrary.BreakRotator` (`self.K2_GetActorRotation`)))
  (bind _gun (`self.Gun`))
  (bind _sprite (`self.Sprite`))
  (bind _sprite_2 (`self.Sprite`))
  (bind (_returnvalue_roll_2 _returnvalue_pitch_2 _returnvalue_yaw) (`KismetMathLibrary.BreakRotator` (`KismetMathLibrary.FindLookAtRotation` (`self.K2_GetActorLocation`) (`.Location` (`GameplayStatics.BreakHitResult` (`PlayerController.GetHitResultUnderCursorByChannel` (`GameplayStatics.GetPlayerController` 0) "TraceTypeQuery1" true))))))
  (`|ExecutionSequence`
    (:`then_0`
      (switch `/Game/E_FaceDirection` (`self.FaceDirection`)
        (:`NewEnumerator0`
          (`SceneComponent.K2_SetRelativeRotation` :`self` _sprite)
          ;[1 1 1] FaceDirection, WeaponDirection
          (if (`self.isBuilding`)
            (`PaperFlipbookComponent.SetFlipbook` _sprite_2 "/Game/Assets/Character/小明_笔记状态_移动动画/小明_移动_笔记_侧上.小明_移动_笔记_侧上")
            (else
              (`PaperFlipbookComponent.SetFlipbook` _sprite_2 "/Game/Assets/Character/小明_攻击状态_移动动画/小明_移动_攻击_侧上.小明_移动_攻击_侧上"))))
        (:`NewEnumerator1`
          (`SceneComponent.K2_SetRelativeRotation` :`self` _sprite)
          (if (`self.isBuilding`)
            (`PaperFlipbookComponent.SetFlipbook` _sprite_2 "/Game/Assets/Character/小明_笔记状态_移动动画/小明_移动_笔记_移动_侧下.小明_移动_笔记_移动_侧下")
            (else
              (`PaperFlipbookComponent.SetFlipbook` _sprite_2 "/Game/Assets/Character/小明_攻击状态_移动动画/小明_移动_攻击_移动_侧下.小明_移动_攻击_移动_侧下"))))
        (:`NewEnumerator2`
          (`SceneComponent.K2_SetRelativeRotation` _sprite (struct :`Yaw` 180.0) false false)
          (if (`self.isBuilding`)
            (`PaperFlipbookComponent.SetFlipbook` _sprite_2 "/Game/Assets/Character/小明_笔记状态_移动动画/小明_移动_笔记_移动_侧下.小明_移动_笔记_移动_侧下")
            (else
              (`PaperFlipbookComponent.SetFlipbook` _sprite_2 "/Game/Assets/Character/小明_攻击状态_移动动画/小明_移动_攻击_移动_侧下.小明_移动_攻击_移动_侧下"))))
        (:`NewEnumerator3`
          (`SceneComponent.K2_SetRelativeRotation` :`self` _sprite)
          (if (`self.isBuilding`)
            (`PaperFlipbookComponent.SetFlipbook` _sprite_2 "/Game/Assets/Character/小明_笔记状态_移动动画/小明_移动_笔记_移动_侧下.小明_移动_笔记_移动_侧下")
            (else
              (`PaperFlipbookComponent.SetFlipbook` _sprite_2 "/Game/Assets/Character/小明_攻击状态_移动动画/小明_移动_攻击_移动_侧下.小明_移动_攻击_移动_侧下"))))
        (:`NewEnumerator4`
          (`SceneComponent.K2_SetRelativeRotation` _sprite (struct :`Yaw` 180.0) false false)
          (if (`self.isBuilding`)
            (`PaperFlipbookComponent.SetFlipbook` _sprite_2 "/Game/Assets/Character/小明_笔记状态_移动动画/小明_移动_笔记_移动_侧下.小明_移动_笔记_移动_侧下")
            (else
              (`PaperFlipbookComponent.SetFlipbook` _sprite_2 "/Game/Assets/Character/小明_攻击状态_移动动画/小明_移动_攻击_侧上.小明_移动_攻击_侧上"))))
        (:`NewEnumerator5`
          (`SceneComponent.K2_SetRelativeRotation` :`self` _sprite)
          (if (`self.isBuilding`)
            (`PaperFlipbookComponent.SetFlipbook` _sprite_2 "/Game/Assets/Character/小明_笔记状态_移动动画/小明_移动_笔记_移动_侧下.小明_移动_笔记_移动_侧下")
            (else
              (`PaperFlipbookComponent.SetFlipbook` _sprite_2 "/Game/Assets/Character/小明_攻击状态_移动动画/小明_移动_攻击_侧上.小明_移动_攻击_侧上"))))
        (:`NewEnumerator6`
          (`SceneComponent.K2_SetRelativeRotation` _sprite (struct :`Yaw` 180.0) false false)
          (if (`self.isBuilding`)
            (`PaperFlipbookComponent.SetFlipbook` _sprite_2 "/Game/Assets/Character/小明_笔记状态_移动动画/小明_移动_笔记_移动_侧下.小明_移动_笔记_移动_侧下")
            (else
              (`PaperFlipbookComponent.SetFlipbook` _sprite_2 "/Game/Assets/Character/小明_攻击状态_移动动画/小明_移动_攻击_移动_侧下.小明_移动_攻击_移动_侧下"))))
        (:`NewEnumerator7`
          (`SceneComponent.K2_SetRelativeRotation` :`self` _sprite)
          (if (`self.isBuilding`)
            (`PaperFlipbookComponent.SetFlipbook` _sprite_2 "/Game/Assets/Character/小明_笔记状态_移动动画/小明_移动_笔记_移动_侧下.小明_移动_笔记_移动_侧下")
            (else
              (`PaperFlipbookComponent.SetFlipbook` _sprite_2 "/Game/Assets/Character/小明_攻击状态_移动动画/小明_移动_攻击_移动_侧下.小明_移动_攻击_移动_侧下"))))))
    (:`then_1`
      ;[1 1 1] TowerRotation Toward Mouse
      (if (`self.isGun`)
        (`SceneComponent.SetVisibility` _gun false false)
        (`SceneComponent.K2_SetWorldRotation` _gun (`KismetMathLibrary.MakeRotator` _returnvalue_roll _returnvalue_pitch _returnvalue_yaw) false false)))))

(fn `UserConstructionScript`)