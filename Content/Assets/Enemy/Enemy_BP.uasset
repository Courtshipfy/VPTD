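; Enemy_BP is a Paper2D enemy that patrols between PointA and PointB via InterpToMovement, flipping its sprite at each reversal.
; Capsule overlap takes 10 Health from the cast character and, if it survives, knocks it back with a sound.
; Tick picks the flipbook from death, damage and velocity state, clears the damage flag after a delay, and at zero Health stops movement, disables collision and triggers death animation and sound.
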(event `self.InterpToMovement.OnInterpToReverse`
  (params (ImpactResult :type "HitResult Structure (by ref)") (Time :type "Float (single-precision)"))
  (bind _paperflipbook (`self.PaperFlipbook`))
  (if (not (`self.IsDead`))
    (`/Engine/EditorBlueprintResources/StandardMacros.FlipFlop`
      (:`A`
        (`SceneComponent.K2_SetWorldRotation` :`self` _paperflipbook))
      (:`B`
        (`SceneComponent.K2_SetWorldRotation` _paperflipbook (struct :`Yaw` 180.0) false false)))))

(event `UpdateAnimation`
  (bind _isdead (`self.IsDead`))
  (if (`self.IsDead`)
    (`/Engine/EditorBlueprintResources/StandardMacros.DoOnce` false
      (:`Completed`
        (`self.Play Death Animation`)))
    (else
      (`PaperFlipbookComponent.SetFlipbook` (`self.PaperFlipbook`) (select `bool` (`self.IsTakingDamage`) :`false` (select `bool` _isdead :`false` (select `bool` (> (`KismetMathLibrary.VSize` (`MovementComponent.Velocity` (`self.InterpToMovement`))) 0.0) :!type "PaperFlipbook Object Reference") :`true` (select `bool` _isdead :!type "PaperFlipbook Object Reference")))))))

(event `self.ReceiveTick`
  (params (DeltaSeconds :type "Float (single-precision)"))
  (bind _interptomovement (`self.InterpToMovement`))
  (`|ExecutionSequence`
    (:`then_0`
      (`self.UpdateAnimation`))
    (:`then_1`
      (`self.PlayDeath` _interptomovement _interptomovement))
    (:`then_2`
      (if (`self.IsTakingDamage`)
        (`KismetSystemLibrary.Delay` 0.6)
        (set `self.IsTakingDamage` false)))))

(event `self.Capsule.OnComponentBeginOverlap`
  (params (OverlappedComponent :type "PrimitiveComponent Object Reference") (OtherActor :type "Actor Object Reference") (OtherComp :type "PrimitiveComponent Object Reference") (OtherBodyIndex :type Integer) (bFromSweep :type Boolean) (SweepResult :type "HitResult Structure (by ref)"))
  (if (not (`self.IsDead`))
    (bind _asplayer_bp (cast `` OtherActor))
    (set `/Game/Assets/Enemy/Enemy_BP.Health` (- (`/Game/Assets/Enemy/Enemy_BP.Health` _asplayer_bp) 10) _asplayer_bp)
    (if (not (`/Game/Assets/Enemy/Enemy_BP.IsDead` _asplayer_bp))
      (`Character.LaunchCharacter` _asplayer_bp (`KismetMathLibrary.MakeVector` (* (.x (`.Normal` (`GameplayStatics.BreakHitResult` SweepResult))) -400.0) 0.0 600.0) true true)
      (`GameplayStatics.SpawnSound2D` null 1.0 1.0 0.0 null))))

(fn `Interp Sprite Rotate`
  (bind _paperflipbook (`self.PaperFlipbook`))
  (if (not (`self.IsDead`))
    (`/Engine/EditorBlueprintResources/StandardMacros.FlipFlop`
      (:`A`
        (`SceneComponent.K2_SetWorldRotation` :`self` _paperflipbook))
      (:`B`
        (`SceneComponent.K2_SetWorldRotation` _paperflipbook (struct :`Yaw` 180.0) false false)))))

(fn `Play Death Animation`
  (bind _paperflipbook (`self.PaperFlipbook`))
  (`PaperFlipbookComponent.SetFlipbook` _paperflipbook null)
  (`PaperFlipbookComponent.SetLooping` _paperflipbook false)
  (`GameplayStatics.SpawnSound2D` "/Engine/EditorSounds/GamePreview/EjectFromPlayer_Cue.EjectFromPlayer_Cue" 1.0 1.0 0.0 null))

(fn `PlayDeath`
  (params (self2 :type "MovementComponent Object Reference") (self3 :type "MovementComponent Object Reference"))
  (if (<= (`KismetMathLibrary.FTrunc` (`self.Health`)) 0)
    (`/Engine/EditorBlueprintResources/StandardMacros.DoOnce` false
      (:`Completed`
        (set `self.IsDead` true)
        (set `MovementComponent.Velocity` (0.0 0.0 0.0) self2)
        (`self.SetActorEnableCollision` false)
        (`MovementComponent.StopMovementImmediately` self3)))))

(fn `UserConstructionScript`
  (set `InterpToMovementComponent.ControlPoints` (`|MakeArray` (make `InterpControlPoint` (`self.PointA`)) (make `InterpControlPoint` (`self.PointB`))) (`self.InterpToMovement`)))