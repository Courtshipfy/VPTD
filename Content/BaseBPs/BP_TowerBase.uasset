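; Tower base actor with a Paper2D sprite that auto-fires projectiles and can be toggled to follow the player.
; VPTDAttribute takes health and level from STTurrent, whose attack speed sets the fire timer, and death destroys the actor.
; When stationary, it sphere-traces for enemies, bubble-sorts them by distance and shoots the nearest.
; Hover tints the sprite, and clicking toggles move mode, where it trails the player and fires toward the mouse cursor.
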(event `self.ReceiveBeginPlay`
  (bind _vptd_attribute (`self.VPTD_Attribute`))
  (bind (_st_turrent_hp _st_turrent_level _st_turrent_damagevalue _st_turrent_attackspeed) (break `ST_Turrent` (`self.ST_Turrent`)))
  (set `VPTD_AttributeComponent.Health` _st_turrent_hp _vptd_attribute)
  (set `VPTD_AttributeComponent.Level` _st_turrent_level _vptd_attribute)
  (`KismetSystemLibrary.K2_SetTimerDelegate` (delegate `FindEnemies`) (/ 1.0 _st_turrent_attackspeed) true)
  (add `self.OnBeginCursorOver` (delegate `Hanging`))
  (add `self.OnEndCursorOver` (delegate `NotHanging`))
  (add `self.OnClicked` (delegate `OnClick`))
  (add `VPTD_AttributeComponent.OnHealthChangedDelegated` (`self.VPTD_Attribute`) (delegate `Die`)))

(event `Die`
  (params (InstigatorActor :type "Actor Object Reference") (OwningComp :type "VPTD_AttributeComponent Object Reference") (NewHealth :type "Float (single-precision)") (Delta :type "Float (single-precision)"))
  (bind _returnvalue (`VPTD_AttributeComponent.IsAlive` (`self.VPTD_Attribute`)))
  (if (not _returnvalue)
    (`KismetSystemLibrary.PrintString` "TestTurrent Die")
    (`self.K2_DestroyActor`)))

(event `Hanging` :!signature `self.OnBeginCursorOver`
  (params (TouchedActor :type "Actor Object Reference"))
  (`PaperSpriteComponent.SetSpriteColor` (`self.PaperSprite`) (make `LinearColor` 1.0 0.0 0.0 0.8)))

(event `NotHanging` :!signature `self.OnEndCursorOver`
  (params (TouchedActor :type "Actor Object Reference"))
  (`PaperSpriteComponent.SetSpriteColor` (`self.PaperSprite`) (make `LinearColor` 1.0 1.0 1.0 1.0)))

(event `OnClick` :!signature `self.OnClicked`
  (params (TouchedActor :type "Actor Object Reference") (ButtonPressed :type "Key Structure" :default "None"))
  (`/Engine/EditorBlueprintResources/StandardMacros.FlipFlop`
    (:`A`
      (set `self.isMove` true))
    (:`B`
      (set `self.isMove` false))))

(event `self.ReceiveTick`
  (params (DeltaSeconds :type "Float (single-precision)"))
  (bind _returnvalue (`self.K2_GetActorLocation`))
  (bind _returnvalue_2 (`self.K2_GetActorLocation` (`GameplayStatics.GetPlayerPawn` 0)))
  ;[1 1 1] 跟随主角
  (if (`self.isMove`)
    (bind _asbp_vptd_game_mode (cast `/Game/BP_VPTD_GameMode` (`GameplayStatics.GetGameMode`)))
    (`/Game/BP_VPTD_GameMode.GetRandomPointInCircle` _asbp_vptd_game_mode (`self.K2_GetActorLocation` (`GameplayStatics.GetPlayerPawn` 0)) (`self.MoveWithDis`))
    (if (not (<= (`KismetMathLibrary.Distance2D` (`KismetMathLibrary.Conv_VectorToVector2D` _returnvalue_2) (`KismetMathLibrary.Conv_VectorToVector2D` _returnvalue)) (`self.MoveWithDis`)))
      (`self.K2_AddActorWorldOffset` (* (- _returnvalue_2 _returnvalue) (* DeltaSeconds 0.5))))))

(event `FindEnemies`
  (bind _returnvalue (`self.K2_GetActorLocation`))
  (bind (_returnvalue_x _returnvalue_y) (`KismetMathLibrary.BreakVector` (`self.K2_GetActorLocation`)))
  (bind _enemiesdistances (`self.EnemiesDistances`))
  (bind _arrayindexes (`self.ArrayIndexes`))
  (bind _arrayindexes_2 (`self.ArrayIndexes`))
  (bind _returnvalue_2 (`KismetArrayLibrary.Array_LastIndex` (`self.EnemiesDistances`)))
  (bind _worldlocation (`PlayerController.DeprojectMousePositionToWorld` (`GameplayStatics.GetPlayerController` 0)))
  (bind (_returnvalue_x_2 _returnvalue_y_2) (`KismetMathLibrary.BreakVector` (- (`self.K2_GetActorLocation`) (`self.K2_GetActorLocation`))))
  (bind (_returnvalue_roll _returnvalue_pitch _returnvalue_yaw) (`KismetMathLibrary.BreakRotator` (`KismetMathLibrary.FindLookAtRotation` (`KismetMathLibrary.MakeVector` _returnvalue_x _returnvalue_y) (`KismetMathLibrary.MakeVector` (.x _worldlocation) (.y _worldlocation)))))
  (bind (_returnvalue_roll_2 _returnvalue_pitch_2 _returnvalue_yaw_2) (`KismetMathLibrary.BreakRotator` (`KismetMathLibrary.FindLookAtRotation` (`self.K2_GetActorLocation`) (`self.K2_GetActorLocation` (`|GetArrayItem` (`self.EnemiesInRange`))))))
  ;[1 1 1] 自动攻击
  ;;[1 1 1] 瞄准开火
  (if (not (`self.isMove`))
    (`|ExecutionSequence`
      (:`then_0`
        (`KismetArrayLibrary.Array_Clear` (`self.EnemiesInRange`))
        (`KismetArrayLibrary.Array_Clear` (`self.EnemiesDistances`))
        (bind _outhits (`KismetSystemLibrary.SphereTraceMultiForObjects` _returnvalue _returnvalue (`self.Range`) (`|MakeArray` "ObjectTypeQuery3" :!type "EObjectTypeQuery Enum")))
        (for _array_element _outhits
          (bind _asbp_enemy_base (cast `/Game/BaseBPs/BP_EnemyBase` (`.HitActor` (`GameplayStatics.BreakHitResult` _array_element))))
          (`KismetArrayLibrary.Array_Add` (`self.EnemiesInRange`) _asbp_enemy_base)))
      (:`then_1`
        (for _array_element_2 (`self.EnemiesInRange`)
          (`KismetArrayLibrary.Array_Add` (`self.EnemiesDistances`) (`KismetMathLibrary.VSizeXY` (- (`self.K2_GetActorLocation` _array_element_2) (`self.K2_GetActorLocation`))))))
      (:`then_2`
        ;;[1 1 1] 冒泡排序
        (set `self.CompareTimes` _returnvalue_2)
        (for _ (range 1 (+ _returnvalue_2 1))
          (set `self.ArrayIndexes` 0)
          (for _ (range 1 (+ (`self.CompareTimes`) 1))
            (if (> (`|GetArrayItem` _enemiesdistances _arrayindexes) (`|GetArrayItem` _enemiesdistances (+ _arrayindexes 1)))
              (`|ExecutionSequence`
                (:`then_0`
                  (`KismetArrayLibrary.Array_Swap` (`self.EnemiesInRange`) _arrayindexes_2 (+ _arrayindexes_2 1)))
                (:`then_1`
                  (`KismetArrayLibrary.Array_Swap` (`self.EnemiesDistances`) _arrayindexes_2 (+ _arrayindexes_2 1))
                  (set `self.CompareTimes` (+ (`self.ArrayIndexes`) 1) :!label _label)))
              (else
                (goto _label))))
          (set `self.CompareTimes` (- (`self.CompareTimes`) 1))))
      (:`then_3`
        (`/Engine/EditorBlueprintResources/StandardMacros.IsValid` (`|GetArrayItem` (`self.EnemiesInRange`))
          (:`Is Valid`
            (`|SpawnActorFromClass` "/Game/BP_TestProjectile.BP_TestProjectile_C" (`KismetMathLibrary.MakeTransform` (- (`self.K2_GetActorLocation`) (* (`KismetMathLibrary.Normal` (`KismetMathLibrary.MakeVector` _returnvalue_x_2 _returnvalue_y_2)) 10.0)) (`KismetMathLibrary.MakeRotator` 0.0 0.0 _returnvalue_yaw_2)) "AdjustIfPossibleButAlwaysSpawn" "MultiplyWithRoot" null null)
            (`KismetSystemLibrary.PrintString` "projectile spwan")))))
    (else
      (`|SpawnActorFromClass` "/Game/BP_TestProjectile.BP_TestProjectile_C" (`KismetMathLibrary.MakeTransform` (`KismetMathLibrary.MakeVector` _returnvalue_x _returnvalue_y 10.0) (`KismetMathLibrary.MakeRotator` 0.0 0.0 (+ _returnvalue_yaw 45.0))) "Undefined" "MultiplyWithRoot" null null))))

(fn `UserConstructionScript`
  (bind (_returnvalue_x _returnvalue_y) (`KismetMathLibrary.BreakVector` (`self.K2_GetActorLocation`)))
  (bind (_returnvalue_roll _returnvalue_pitch _returnvalue_yaw) (`KismetMathLibrary.BreakRotator` (`self.K2_GetActorRotation`)))
  (`self.K2_SetActorLocation` (`KismetMathLibrary.MakeVector` _returnvalue_x _returnvalue_y 10.0))
  (`self.K2_SetActorRotation` (`KismetMathLibrary.MakeRotator` -90.0 _returnvalue_pitch _returnvalue_yaw)))