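; Base enemy Blueprint that chases the player, deals contact damage and drops loot, tuned by the STEnemyAttributes struct.
; When IsMoving is set, Tick offsets it toward the player without sweep or normalization, so speed grows with distance.
; Capsule overlap damages any actor with an attributes component.
; Any health change with non-positive Delta triggers death, spawning scattered money and exp pickups, with DestroyActor called inside the exp loop.
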(event `self.ReceiveBeginPlay`
  (bind (_st_enemyattributes_moneynum _st_enemyattributes_expnum _st_enemyattributes_money _st_enemyattributes_exp _st_enemyattributes_hp _st_enemyattributes_movespeed _st_enemyattributes_damagevalue) (break `ST_Enemy` (`self.ST_EnemyAttributes`)))
  (add `VPTD_AttributeComponent.OnHealthChangedDelegated` (`self.VPTDAttribute`) (delegate `Die`))
  (set `VPTD_AttributeComponent.HealthMax` _st_enemyattributes_hp (`self.VPTDAttribute`)))

(event `Die`
  (params (InstigatorActor :type "Actor Object Reference") (OwningComp :type "VPTD_AttributeComponent Object Reference") (NewHealth :type "Float (single-precision)") (Delta :type "Float (single-precision)"))
  (bind _returnvalue (`KismetMathLibrary.RandomIntegerInRange` 1 5))
  (bind _returnvalue_2 (`self.K2_GetActorLocation`))
  (bind (_st_enemyattributes_moneynum _st_enemyattributes_expnum _st_enemyattributes_money _st_enemyattributes_exp _st_enemyattributes_hp _st_enemyattributes_movespeed _st_enemyattributes_damagevalue) (break `ST_Enemy` (`self.ST_EnemyAttributes`)))
  (if (<= Delta 0.0)
    (`KismetSystemLibrary.PrintString` "enemy dead" true true (struct :`R` 1.0 :`B` 0.315367 :`A` 1.0))
    (for _index (range 1 (+ _st_enemyattributes_moneynum 1))
      (`|SpawnActorFromClass` "/Game/BP_ItemMoney.BP_ItemMoney_C" (`KismetMathLibrary.MakeTransform` (- _returnvalue_2 (`KismetMathLibrary.MakeVector` _returnvalue _returnvalue))) "Undefined" "MultiplyWithRoot" null null))
    (for _index_2 (range 1 (+ _st_enemyattributes_expnum 1))
      (bind _returnvalue_3 (* _index_2 (`KismetMathLibrary.RandomIntegerInRange` 1 5)))
      (`|SpawnActorFromClass` "/Game/BP_ItemExp.BP_ItemExp_C" (`KismetMathLibrary.MakeTransform` (+ (`KismetMathLibrary.MakeVector` _returnvalue_3 _returnvalue_3) _returnvalue_2)) "Undefined" "MultiplyWithRoot" null null)
      (`self.K2_DestroyActor`))))

(event `self.ReceiveTick`
  (params (DeltaSeconds :type "Float (single-precision)"))
  (bind (_st_enemyattributes_moneynum _st_enemyattributes_expnum _st_enemyattributes_money _st_enemyattributes_exp _st_enemyattributes_hp _st_enemyattributes_movespeed _st_enemyattributes_damagevalue) (break `ST_Enemy` (`self.ST_EnemyAttributes`)))
  (if (`self.isMoving`)
    (`self.K2_AddActorWorldOffset` (* (- (`self.K2_GetActorLocation` (`GameplayStatics.GetPlayerPawn` 0)) (`self.K2_GetActorLocation`)) (* DeltaSeconds _st_enemyattributes_movespeed)))))

(event `self.CapsuleComponent.OnComponentBeginOverlap`
  (params (OverlappedComponent :type "PrimitiveComponent Object Reference") (OtherActor :type "Actor Object Reference") (OtherComp :type "PrimitiveComponent Object Reference") (OtherBodyIndex :type Integer) (bFromSweep :type Boolean) (SweepResult :type "HitResult Structure (by ref)"))
  (bind (_st_enemyattributes_moneynum _st_enemyattributes_expnum _st_enemyattributes_money _st_enemyattributes_exp _st_enemyattributes_hp _st_enemyattributes_movespeed _st_enemyattributes_damagevalue) (break `ST_Enemy` (`self.ST_EnemyAttributes`)))
  (bind _returnvalue (`VPTD_AttributeComponent.GetAttributes` OtherActor))
  (`/Engine/EditorBlueprintResources/StandardMacros.IsValid` _returnvalue
    (:`Is Valid`
      (`VPTD_AttributeComponent.ApplyChangeHealth` _returnvalue null (- 0.0 _st_enemyattributes_damagevalue))
      (`KismetSystemLibrary.PrintString` (`KismetSystemLibrary.GetDisplayName` OtherActor)))))

(fn `UserConstructionScript`
  (`parent.UserConstructionScript`))