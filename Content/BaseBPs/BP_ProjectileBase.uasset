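; Base projectile actor that damages enemies on contact.
; Construction pins it to a fixed world height and roll, and BeginPlay sets its local-space ProjectileMovement velocity from ProjectileSpeed.
; A sphere overlap with a BP_EnemyBase subtracts fixed health through the enemy's attributes, then destroys the projectile.
; The timed self-destroy is unconnected, so this graph never removes projectiles that miss.
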(event `self.ReceiveBeginPlay`
  (`ProjectileMovementComponent.SetVelocityInLocalSpace` (`self.ProjectileMovement`) (`KismetMathLibrary.Conv_DoubleToVector` (`self.ProjectileSpeed`))))

(event `self.Sphere.OnComponentBeginOverlap`
  (params (OverlappedComponent :type "PrimitiveComponent Object Reference") (OtherActor :type "Actor Object Reference") (OtherComp :type "PrimitiveComponent Object Reference") (OtherBodyIndex :type Integer) (bFromSweep :type Boolean) (SweepResult :type "HitResult Structure (by ref)"))
  (cast `/Game/BaseBPs/BP_EnemyBase` OtherActor)
  (bind _returnvalue (`VPTD_AttributeComponent.GetAttributes` OtherActor))
  (`VPTD_AttributeComponent.ApplyChangeHealth` _returnvalue null -100.0)
  (`self.K2_DestroyActor`))

(fn `UserConstructionScript`
  (bind (_returnvalue_x _returnvalue_y) (`KismetMathLibrary.BreakVector` (`self.K2_GetActorLocation`)))
  (bind (_returnvalue_roll _returnvalue_pitch _returnvalue_yaw) (`KismetMathLibrary.BreakRotator` (`self.K2_GetActorRotation`)))
  (`self.K2_SetActorLocation` (`KismetMathLibrary.MakeVector` _returnvalue_x _returnvalue_y 10.0))
  (`self.K2_SetActorRotation` (`KismetMathLibrary.MakeRotator` -90.0 _returnvalue_pitch _returnvalue_yaw)))