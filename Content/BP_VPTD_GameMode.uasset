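; Game mode that runs the session: mouse-driven HUD, enemy spawning, level-up feedback and game over.
; On BeginPlay it adds the attributes widget and binds the player's health and level delegates, which trigger the level-up display or freeze time and show an end screen at zero health.
; A looping timer spawns test enemies near the player, offsetting X and Y by independently randomized angles.
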(event `self.ReceiveBeginPlay`
  (bind _returnvalue (`GameplayStatics.GetPlayerController` 0))
  (set `PlayerController.bShowMouseCursor` true _returnvalue)
  (set `PlayerController.bEnableClickEvents` true _returnvalue)
  (set `PlayerController.bEnableMouseOverEvents` true _returnvalue)
  (`|ExecutionSequence`
    (:`then_0`
      (bind _returnvalue_2 (`|CreateWidget` "/Game/Blueprint/Widgets_BP/Attributes_Widget.Attributes_Widget_C"))
      (`UserWidget.AddToViewport` _returnvalue_2 0)
      (bind _returnvalue_3 (`VPTD_AttributeComponent.GetAttributes` (`GameplayStatics.GetPlayerPawn` 0)))
      (add `VPTD_AttributeComponent.OnHealthChangedDelegated` _returnvalue_3 (delegate `GameOver`))
      (add `VPTD_AttributeComponent.OnLevelChangedDelegated` _returnvalue_3 (delegate `LevelUp`)))
    (:`then_1`
      (`KismetSystemLibrary.K2_SetTimerDelegate` (delegate `SpawnEnemy`) 1.0 true))))

(event `GameOver`
  (params (InstigatorActor :type "Actor Object Reference") (OwningComp :type "VPTD_AttributeComponent Object Reference") (NewHealth :type "Float (single-precision)") (Delta :type "Float (single-precision)"))
  (if (<= NewHealth 0.0)
    (`GameplayStatics.SetGlobalTimeDilation` 0.0)
    (bind _returnvalue (`|CreateWidget` "/Game/Blueprint/Widgets_BP/UI_结束画面.UI_结束画面_C"))
    (`UserWidget.AddToViewport` _returnvalue 0)))

(event `LevelUp`
  (params (InstigatorActor :type "Actor Object Reference") (OwningComp :type "VPTD_AttributeComponent Object Reference") (Delta :type Integer))
  (bind _foundwidgets (`WidgetBlueprintLibrary.GetAllWidgetsOfClass` "/Game/Blueprint/Widgets_BP/Attributes_Widget.Attributes_Widget_C"))
  (`/Game/Blueprint/Widgets_BP/Attributes_Widget.ShowLevelUp` (`|GetArrayItem` _foundwidgets)))

(event `SpawnEnemy`
  (bind _randomlocation (`self.GetRandomPointInCircle` (`self.K2_GetActorLocation` (`GameplayStatics.GetPlayerPawn` 0)) 100.0))
  (bind _output_get (set `self.SpawnLocation` _randomlocation))
  (`|SpawnActorFromClass` "/Game/BP_TestEnemy.BP_TestEnemy_C" (`KismetMathLibrary.MakeTransform` _output_get) "Undefined" "MultiplyWithRoot" null null))

(fn `GetRandomPointInCircle`
  (params (Location :type "Vector Structure") (Radius :type "Float (double-precision)"))
  (returns (RandomLocation :type "Vector Structure"))
  (bind _returnvalue (`KismetMathLibrary.DegreesToRadians` (`KismetMathLibrary.RandomFloatInRange` 0.0 360.0)))
  (return (`KismetMathLibrary.MakeVector` (+ Location_X (* Radius (`KismetMathLibrary.Sin` _returnvalue))) (+ Location_Y (* Radius (`KismetMathLibrary.Cos` _returnvalue))) Location_Z)))

(fn `UserConstructionScript`)